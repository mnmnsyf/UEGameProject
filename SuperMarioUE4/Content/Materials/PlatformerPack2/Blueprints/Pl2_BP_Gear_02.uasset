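; Platformer gear actor that spins continuously while bobbing up and down along its local Z axis.
; BeginPlay picks a random starting vertical direction.
; Each Tick applies a fixed local yaw step and a non-swept vertical offset, while a latent Delay in the same Tick flips the direction every few seconds.
; Both motions are per-frame steps, so their speed depends on frame rate.
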(event EventBeginPlay
  (Variables|Default|SetUpOrDown (Math|Random|RandomBool)))

(event EventTick
  (params (DeltaSeconds :type Float%20%28single-precision%29))
  (Utilities|FlowControl|Sequence
    (:then_0
      ;[1 1 1] Makes the Gear rotate by .25 degrees each Event Tick
      (Transformation|AddActorLocalRotation "0,0.250000, 0" false false))
    (:then_1
      (if (Variables|Default|GetUpOrDown)
        (Transformation|AddActorLocalOffset "0, 0,-2.000000" false false)
        (Utilities|FlowControl|Delay 3.0)
        (Variables|Default|SetUpOrDown false)
        (else
          (Transformation|AddActorLocalOffset "0, 0,2.000000" false false)
          (Utilities|FlowControl|Delay 3.0)
          (Variables|Default|SetUpOrDown true))))))

(fn ConstructionScript)