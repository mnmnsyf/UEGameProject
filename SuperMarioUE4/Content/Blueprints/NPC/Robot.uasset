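; Robot NPC that shows dialogue on screen, with lines that depend on whether the player has the key.
; ShowDialogue creates a Conversation_Robot widget that references the robot, then advances DialogueIndex; HideDialogue removes the widget.
; The GetKey flag on MyPlayerState picks the loop: the first three indices without the key, or index two through the last entry with it.
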(event EventBeginPlay)

(event Collision|EventActorBeginOverlap
  (params (OtherActor :type Actor%20Object%20Reference)))

(event EventTick
  (params (DeltaSeconds :type Float%20%28single-precision%29)))

(fn ConstructionScript)

(fn ShowDialogue
  (bind _returnvalue (UserInterface|CreateWidget "/Game/Blueprints/UI/Conversation_Robot.Conversation_Robot_C" 0 self))
  (bind _output_get (Variables|Default|SetDialogueWidget _returnvalue))
  (UserInterface|Viewport|AddtoViewport _output_get 0)
  (if (Variables|/Game/GamePlay/MyPlayerState.MyPlayerState_C|GetGetKey? (.AsMy%20Player%20State (Utilities|Casting|CastToMyPlayerState (Variables|/Script/Engine.Pawn|GetPlayerState (Game|GetPlayerCharacter 0)))))
    (if (>= (Variables|Default|GetDialogueIndex) (Utilities|Array|LastIndex (Variables|Default|GetDialogue)))
      (Variables|Default|SetDialogueIndex 2)
      (else
        (Variables|Default|SetDialogueIndex (+ (Variables|Default|GetDialogueIndex) 1))))
    (elif (>= (Variables|Default|GetDialogueIndex) 2)
      (Variables|Default|SetDialogueIndex 0)
      (else
        (Variables|Default|SetDialogueIndex (+ (Variables|Default|GetDialogueIndex) 1))))))

(fn HideDialogue
  (Widget|RemovefromParent (Variables|Default|GetDialogueWidget)))